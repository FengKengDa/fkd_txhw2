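; Countdown Blueprint that prints the remaining time on screen and ends with a "Game Over" message.
; Tick feeds a one-second Delay, which ignores calls while pending and so paces the countdown to roughly once per second.
; While the integer value of Time is above zero, each step decrements it, then prints the new value or "Game Over" once it runs out.
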(event `self.ReceiveTick`
  (params (DeltaSeconds :type "Float (single-precision)"))
  (`KismetSystemLibrary.Delay` 1.0)
  (`/Engine/EditorBlueprintResources/StandardMacros.CompareInt` (`KismetMathLibrary.Conv_ByteToInt` (`self.time`))
    (:`>`
      (bind _output_get (set `self.time` (- (`self.time`) 1)))
      (if (> (`self.time`) 0)
        (`KismetSystemLibrary.PrintString` (`KismetStringLibrary.Conv_ByteToString` _output_get) true true (struct :`G` 0.66 :`B` 1.0 :`A` 1.0) 1.0)
        (else
          (`KismetSystemLibrary.PrintString` "Game Over"))))))

(fn `UserConstructionScript`)